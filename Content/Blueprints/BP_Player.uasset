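; Player actor that moves in fixed steps, turns 90 degrees at a time and triggers one timed ability, levitation or global time slowdown.
; Enhanced Input drives it, with a Side flag flipped on each turn to choose the axis of the swept step.
; A per-tick downward trace picks the height restored after levitation and snaps Z when ground is distant and no ability runs.
; Custom events reload MainLevel or quit the game.
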(event `self.ReceiveBeginPlay`
  (bind _asplayer_controller (cast `PlayerController` (`self.GetController`)))
  (bind _returnvalue (pcsubsystem `EnhancedInputLocalPlayerSubsystem` _asplayer_controller))
  (`/Engine/EditorBlueprintResources/StandardMacros.IsValid` _returnvalue
    (:`Is Valid`
      (`EnhancedInputSubsystemInterface.AddMappingContext` _returnvalue "/Game/Input/IMC_MyGame.IMC_MyGame" 0 (struct)))))

(event `EnhancedInput|/Game/Input/IA_Move`
  (params (ActionValue :type "Vector2D Structure") (ElapsedSeconds :type "Float (double-precision)") (TriggeredSeconds :type "Float (double-precision)") (InputAction :type "InputAction Object Reference" :default "/Game/Input/IA_Move.IA_Move"))
  (bind _returnvalue (`self.GetActorForwardVector`))
  (bind _returnvalue_2 (`self.K2_GetActorLocation`))
  (bind _side (`self.Side`))
  (:`Started`
    (if (== ActionValue_X 1.0)
      (if _side
        (`self.K2_SetActorLocation` (+ _returnvalue_2 (* _returnvalue (0.0 100.0 0.0))) true)
        (else
          (`self.K2_SetActorLocation` (+ _returnvalue_2 (* _returnvalue (100.0 0.0 0.0))) true)))
      (elif _side
        (`self.K2_SetActorLocation` (+ _returnvalue_2 (* _returnvalue (0.0 -100.0 0.0))) true)
        (else
          (`self.K2_SetActorLocation` (+ _returnvalue_2 (* _returnvalue (-100.0 0.0 0.0))) true))))))

(event `EnhancedInput|/Game/Input/IA_Rotate`
  (params (ActionValue :type "Vector2D Structure") (ElapsedSeconds :type "Float (double-precision)") (TriggeredSeconds :type "Float (double-precision)") (InputAction :type "InputAction Object Reference" :default "/Game/Input/IA_Rotate.IA_Rotate"))
  (bind _returnvalue (`self.K2_GetActorRotation`))
  (:`Started`
    (if (== ActionValue_X 1.0)
      (`self.K2_SetActorRotation` (`KismetMathLibrary.MakeRotator` (.roll _returnvalue) (.pitch _returnvalue) (+ (.yaw _returnvalue) 90.0)))
      (else
        (`self.K2_SetActorRotation` (`KismetMathLibrary.MakeRotator` (.roll _returnvalue) (.pitch _returnvalue) (- (.yaw _returnvalue) 90.0)))))
    (if (`self.Side`)
      (set `self.Side` false)
      (else
        (set `self.Side` true)))))

(event `EnhancedInput|/Game/Input/IA_Ability`
  (params (ActionValue :type Boolean) (ElapsedSeconds :type "Float (double-precision)") (TriggeredSeconds :type "Float (double-precision)") (InputAction :type "InputAction Object Reference" :default "/Game/Input/IA_Ability.IA_Ability"))
  (bind (_returnvalue_x _returnvalue_y _returnvalue_z) (`KismetMathLibrary.BreakVector` (`self.K2_GetActorLocation`)))
  (:`Started`
    (if (== (`self.CurrentAbility`) "Levitation")
      (if (not (`self.isAbilityActive`))
        (`self.K2_SetActorLocation` (`KismetMathLibrary.MakeVector` _returnvalue_x _returnvalue_y (`self.LevitationHeight`)))
        (set `self.isAbilityActive` true)
        (`KismetSystemLibrary.K2_SetTimer` null "EndLevitation" (`self.AbilityDuration`)))
      (elif (== (`self.CurrentAbility`) "TimeSlowdown")
        (if (not (`self.isAbilityActive`))
          (`GameplayStatics.SetGlobalTimeDilation` (`self.TimeDilationAmount`))
          (set `self.isAbilityActive` true)
          (`KismetSystemLibrary.K2_SetTimer` null "EndTimeSlowdown" (- (`self.AbilityDuration`) 3.5)))))))

(event `self.ReceiveActorBeginOverlap`
  (params (OtherActor :type "Actor Object Reference")))

(event `self.ReceiveTick`
  (params (DeltaSeconds :type "Float (single-precision)"))
  (bind _returnvalue (`self.K2_GetActorLocation`))
  (bind (_returnvalue_x _returnvalue_y) (`KismetMathLibrary.BreakVector` (`self.K2_GetActorLocation`)))
  (bind (_returnvalue_x_2 _returnvalue_y_2 _returnvalue_z) (`KismetMathLibrary.BreakVector` (`self.K2_GetActorLocation`)))
  (bind _outhit (`KismetSystemLibrary.LineTraceSingle` _returnvalue (- _returnvalue (0.0 0.0 1000.0)) "TraceTypeQuery1"))
  (bind _output_get (set `self.GroundDIstance` (- _returnvalue_z (.z (`.Location` (`GameplayStatics.BreakHitResult` _outhit))))))
  (if (>= _output_get 150.0)
    (bind _output_get_2 (set `self.OriginalHeight` 100.0))
    (if (not (`self.isAbilityActive`))
      (`self.K2_SetActorLocation` (`KismetMathLibrary.MakeVector` _returnvalue_x _returnvalue_y _output_get_2)))
    (else
      (set `self.OriginalHeight` 200.0))))

(event `TeleportPlayerBack`
  (`GameplayStatics.OpenLevel` "MainLevel"))

(event `EndGame`
  (`KismetSystemLibrary.QuitGame` null "Quit"))

(fn `EndLevitation`
  (bind (_returnvalue_x _returnvalue_y) (`KismetMathLibrary.BreakVector` (`self.K2_GetActorLocation`)))
  (`self.K2_SetActorLocation` (`KismetMathLibrary.MakeVector` _returnvalue_x _returnvalue_y (`self.OriginalHeight`)))
  (set `self.isAbilityActive` false)
  (if (not (== (`self.CurrentAbility`) "TimeSlowdown"))
    (set `self.CurrentAbility` "None")))

(fn `EndTimeSlowdown`
  (`GameplayStatics.SetGlobalTimeDilation` 1.0)
  (set `self.isAbilityActive` false)
  (set `self.CurrentAbility` "None"))

(fn `UserConstructionScript`)